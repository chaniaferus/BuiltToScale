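; BP_Laser is an art actor that gently sways in position and pitch, presumably as an animated laser prop.
; BeginPlay stores the starting XY and randomizes phase, frequency and amplitude so instances move out of sync.
; Tick applies time-based sines: X and Y share one offset, giving diagonal drift, while Z, roll and yaw are preserved.
; Pitch swings by a fixed amplitude, leaving the randomized rotation amplitude unused.
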(event EventBeginPlay
  (bind _returnvalue (Transformation|GetActorLocation))
  (Variables|Default|SetInitX (.x _returnvalue))
  (Variables|Default|SetInitY (.y _returnvalue))
  (Variables|Default|SetRandomOffset (Math|Random|RandomFloatinRange 0.0 1.0))
  (Variables|Default|SetRandomRotOffset (Math|Random|RandomFloatinRange 0.0 1.0))
  (Variables|Default|SetRandomFreq (Math|Random|RandomFloatinRange 0.1 0.25))
  (Variables|Default|SetRandomAplitude (Math|Random|RandomFloatinRange 1.5 2.5))
  (Variables|Default|SetRandomRotAmplitude (Math|Random|RandomFloatinRange 1e+01 25.0)))

(event EventTick
  (params (DeltaSeconds :type Float%20%28single-precision%29))
  (bind _returnvalue (Transformation|GetActorRotation))
  (bind _returnvalue_2 (Utilities|Time|GetGameTimeinSeconds))
  (bind _randomoffset (Variables|Default|GetRandomOffset))
  (bind _randomaplitude (Variables|Default|GetRandomAplitude))
  (bind _randomfreq (Variables|Default|GetRandomFreq))
  (bind _returnvalue_3 (+ _randomoffset _returnvalue_2))
  (bind _returnvalue_4 (* _returnvalue_3 _randomfreq))
  (bind _returnvalue_5 (Math|Trig|Sin(Radians) _returnvalue_4))
  (bind _returnvalue_6 (* _randomaplitude _returnvalue_5))
  (Transformation|SetActorLocationAndRotation (Math|Vector|MakeVector (+ (Variables|Default|GetInitX) _returnvalue_6) (+ (Variables|Default|GetInitY) _returnvalue_6) (.z (Transformation|GetActorLocation))) (Math|Rotator|MakeRotator (.roll _returnvalue) (* (Math|Trig|Sin(Radians) (* _randomfreq (+ _returnvalue_2 (Variables|Default|GetRandomRotOffset)))) 3e+01) (.yaw _returnvalue))))

(fn ConstructionScript)