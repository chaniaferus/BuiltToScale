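; BP_MusicPlane is a music-reactive plane that plays a track and pulses its grid material with the loudness.
; The construction script takes the sound and duration from a LoudnessAnalyzer asset, keeping audio and precomputed analysis matched.
; Playback-percent callbacks look up normalized loudness at the current time and drive the dynamic material's Intensity, with a minimum floor.
; Tick scrolls the material's UV offsets with game time, V at half U's speed.
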(event Custom|OnAudioPlaybackPercent_Event
  (params (PlayingSoundWave :type Sound%20Wave%20Object%20Reference) (PlaybackPercent :type Float%20%28single-precision%29))
  (bind _remainder (Math|Float|Division(WholeandRemainder) PlaybackPercent 1e+02))
  (bind _duration (Variables|Default|Getduration))
  (bind _loudnessanalyzer (Variables|Default|GetLoudnessAnalyzer))
  (bind _material (Variables|Default|GetMaterial))
  (bind _returnvalue (* _remainder _duration))
  (bind _outloudness (Class|LoudnessNRT|GetNormalizedLoudnessatTime _loudnessanalyzer _returnvalue))
  (if (> _outloudness 0.1)
    (Rendering|Material|SetScalarParameterValue _material "Intensity" _outloudness :!class /Script/Engine.MaterialInstanceDynamic)
    (else
      (Rendering|Material|SetScalarParameterValue _material "Intensity" 0.1 :!class /Script/Engine.MaterialInstanceDynamic))))

(event EventBeginPlay
  (bind _audio (Variables|Default|GetAudio))
  (bind _returnvalue (Rendering|Material|CreateDynamicMaterialInstance (Variables|Default|GetPlane) 0 "/Game/Art/GridMaterial.GridMaterial" "None" :!class /Script/Engine.PrimitiveComponent))
  (bind _output_get (Variables|Default|SetMaterial _returnvalue))
  (Rendering|Material|SetMaterial (Variables|Default|GetPlane) 0 _output_get)
  (EventDispatchers|AssignOnAudioPlaybackPercent (Variables|Default|GetAudio) (delegate Custom|OnAudioPlaybackPercent_Event))
  (Audio|Components|Audio|SetVolumeMultiplier _audio 1.0 :!class /Script/Engine.AudioComponent)
  (Audio|Components|Audio|Play _audio 0.0))

(event Collision|EventActorBeginOverlap
  (params (OtherActor :type Actor%20Object%20Reference)))

(event EventTick
  (params (DeltaSeconds :type Float%20%28single-precision%29))
  (bind _returnvalue (Utilities|Time|GetGameTimeinSeconds))
  (bind _material (Variables|Default|GetMaterial))
  (bind _returnvalue_2 (/ _returnvalue 2e+01))
  (Rendering|Material|SetScalarParameterValue _material "U Offset" _returnvalue_2 :!class /Script/Engine.MaterialInstanceDynamic)
  (Rendering|Material|SetScalarParameterValue _material "V Offset" (/ _returnvalue_2 2.0) :!class /Script/Engine.MaterialInstanceDynamic))

(fn ConstructionScript
  (bind _loudnessanalyzer (Variables|Default|GetLoudnessAnalyzer))
  (bind _sound (Variables|/Script/AudioAnalyzer.AudioAnalyzerNRT|GetSound _loudnessanalyzer))
  (Audio|Components|Audio|SetSound (Variables|Default|GetAudio) _sound)
  (Variables|Default|Setduration (Variables|/Script/Engine.SoundBase|GetDuration _sound)))