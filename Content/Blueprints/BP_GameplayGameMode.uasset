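; Game mode for a Tetris-style game that handles scoring, level progression and difficulty.
; Score scales with the square of lines cleared, the area width and a multiplier summed from the spawner's unlocked block classes.
; Score thresholds raise the level and randomly widen or heighten the BP_GameArea found at BeginPlay.
; Every other level shortens the move interval within limits and pauses the game for the block swap widget.
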(event EventBeginPlay
  (bind _outactors (Actor|GetAllActorsOfClass "/Game/Blueprints/BP_GameArea.BP_GameArea_C"))
  (Variables|Default|SetGameAreaRef (Utilities|Array|Get(acopy) _outactors)))

(event EventTick
  (params (DeltaSeconds :type Float%20%28single-precision%29)))

(fn ConstructionScript)

(fn CalculateScore
  (params (LinesCleared :type Integer))
  (bind _difficultymultiplier (Variables|Default|GetDifficultyMultiplier))
  (Variables|Default|SetScore (+ (Variables|Default|GetScore) (* (* LinesCleared (* (Variables|Default|GetPointsPerBlock) (* LinesCleared (Variables|/Game/Blueprints/BP_GameArea.BP_GameArea_C|GetSizeX (Variables|Default|GetGameAreaRef))))) _difficultymultiplier)))
  (Development|PrintString (Utilities|String|ToString(Float) _difficultymultiplier))
  (CallFunction|UpdateLevelScale))

(fn UpdateLevelScale
  (bind _returnvalue (Game|GetPlayerController 0))
  (bind _gamearearef (Variables|Default|GetGameAreaRef))
  (if (>= (Variables|Default|GetScore) (Variables|Default|GetNextUpdateTreshold))
    (Utilities|FlowControl|Sequence
      (:then_0
        (if (Math|Random|RandomBool)
          (LocalVariables|SetAddition 2.0)
          (else
            (LocalVariables|SetAddition 4.0)))
        (if (Math|Random|RandomBool)
          (Variables|/Game/Blueprints/BP_GameArea.BP_GameArea_C|SetSizeY _gamearearef (+ (Variables|/Game/Blueprints/BP_GameArea.BP_GameArea_C|GetSizeY _gamearearef) (LocalVariables|GetAddition)))
          (else
            (Variables|/Game/Blueprints/BP_GameArea.BP_GameArea_C|SetSizeX _gamearearef (+ (Variables|/Game/Blueprints/BP_GameArea.BP_GameArea_C|GetSizeX _gamearearef) (LocalVariables|GetAddition)))))
        (Default|ScaleBorders _gamearearef))
      (:then_1
        (Variables|Default|SetNextUpdateTreshold (+ (Variables|Default|GetNextUpdateTreshold) 300))
        (bind _result (Math|Integer|IncrementInt (Variables|Default|GetPlayerLevel))
          (:%20%20
            (if (== (Math|Integer|%(Integer) _result 2) 0)
              (Variables|Default|SetMoveInterval (Math|Float|Clamp(Float) (- (Variables|Default|GetMoveInterval) 0.05) 0.1 0.5))
              (Game|SetGamePaused true)
              (bind _returnvalue_2 (UserInterface|CreateWidget "/Game/UI/WBP_BlockSwap.WBP_BlockSwap_C" _returnvalue))
              (UserInterface|Viewport|AddtoViewport _returnvalue_2 0)
              (Input|SetInputModeUIOnly _returnvalue _returnvalue_2 "DoNotLock" true)
              (Variables|/Script/Engine.PlayerController|SetbShowMouseCursor _returnvalue true))))))))

(fn CalculateDifficultyMultiplier
  (for _array_element (Variables|/Script/BuiltToScale.BlockSpawner|GetUnlockedBlocks (Subsystems|GetBlockSpawner))
    (bind _asbp_tetromino (Utilities|Casting|CastToBP_TetrominoClass _array_element))
    (LocalVariables|SetLocalMultiplier (+ (LocalVariables|GetLocalMultiplier) (.MultiplierAdditive (Utilities|GetClassDefaults _asbp_tetromino)))))
  (Variables|Default|SetDifficultyMultiplier (LocalVariables|GetLocalMultiplier)))