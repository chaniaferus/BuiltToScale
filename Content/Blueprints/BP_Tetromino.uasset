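; BP_Tetromino is a falling Tetris-style piece that can shift sideways, rotate in 90-degree steps and drop.
; A looping timer at the game mode's MoveInterval steps it down.
; Each move applies first, then reverts if per-mesh box overlaps hit WorldStatic objects.
; After a blocked drop, the next tick replaces each mesh with a BP_SingleBlock of matching material, requests a new piece and destroys the actor.
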(event Custom|ProcessBlock
  (if (Variables|Default|GetShouldDrop)
    (CallFunction|TryDropBlock)
    (else
      (Utilities|Time|ClearandInvalidateTimerbyHandle (Variables|Default|GetTimerHandle))
      (for _array_element (Actor|GetComponentsByClass "/Script/Engine.StaticMeshComponent")
        (Game|SpawnActorfromClass "/Game/Blueprints/Blocks/BP_SingleBlock.BP_SingleBlock_C" (Transformation|GetWorldTransform _array_element) "Undefined" "MultiplyWithRoot" 0 (Rendering|Material|GetMaterial _array_element 0) 0))
      (Class|BlockSpawner|SpawnBlock (Subsystems|GetBlockSpawner))
      (Actor|DestroyActor))))

(event EventBeginPlay
  (bind _asbp_gameplay_game_mode (Utilities|Casting|CastToBP_GameplayGameMode (Game|GetGameMode)))
  (bind _returnvalue (Utilities|Time|SetTimerbyEvent (delegate Custom|ProcessBlock) (Variables|/Script/BuiltToScale.BlockGameMode|GetMoveInterval _asbp_gameplay_game_mode) true))
  (Variables|Default|SetTimerHandle _returnvalue))

(fn ConstructionScript)

(fn TryMove
  (params (MoveDirection :type Float%20%28double-precision%29))
  (bind _movedistance (Variables|Default|GetMoveDistance))
  (bind _returnvalue (* MoveDirection _movedistance))
  (LocalVariables|SetLocalMoveDistance _returnvalue)
  (Transformation|AddActorWorldOffset (Math|Vector|MakeVector 0.0 _returnvalue 0.0))
  (bind _didcollide (CallFunction|ChackColision))
  (if _didcollide
    (Transformation|AddActorWorldOffset (Math|Vector|MakeVector 0.0 (* (LocalVariables|GetLocalMoveDistance) -1.0) 0.0))))

(fn TryRotate
  (params (Direction :type Float%20%28double-precision%29))
  (bind _output_get (LocalVariables|SetLocalDeltaRotation (* "0.000000,0.000000,90.000000" Direction)))
  (Class|Actor|AddActorWorldRotation _output_get)
  (bind _didcollide (CallFunction|ChackColision))
  (if _didcollide
    (Class|Actor|AddActorWorldRotation (* (LocalVariables|GetLocalDeltaRotation) -1.0))))

(fn TryDropBlock
  (if (Variables|Default|GetShouldDrop)
    (Transformation|AddActorWorldOffset (Math|Vector|MakeVector 0.0 0.0 (* (Variables|Default|GetMoveDistance) -1.0)) true)
    (bind _didcollide (CallFunction|ChackColision))
    (if _didcollide
      (Transformation|AddActorWorldOffset (Math|Vector|MakeVector 0.0 0.0 (Variables|Default|GetMoveDistance)) true)
      (Variables|Default|SetShouldDrop false))))

(fn ChackColision
  (bind _array_element (Utilities|Array|ForEachLoopwithBreak (Actor|GetComponentsByClass "/Script/Engine.StaticMeshComponent") :!label _label)
    (:LoopBody
      (bind _returnvalue (Collision|BoxOverlapActors (Transformation|GetWorldLocation _array_element) "20.000000,20.000000,20.000000" (Utilities|Array|MakeArray "ObjectTypeQuery1") 0 :!class /Script/Engine.KismetSystemLibrary))
      (bind _output_get (LocalVariables|SetDidHit _returnvalue))
      (if _output_get
        (goto _label Break)))
    (:Completed
      (return (LocalVariables|GetDidHit)))))