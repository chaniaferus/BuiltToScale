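; Player controller for a Tetris-style game that turns Enhanced Input into commands for the falling tetromino.
; It adds the default mapping context on BeginPlay, then forwards move, rotate and hard-drop presses to the block spawner's active tetromino.
; Holding move-down speeds up play by raising global time dilation and restores it on release.
; The main menu input is bound but does nothing.
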(event Input|EnhancedActionEvents|EnhancedInputActionIA_MoveDown
  (params (ActionValue :type Boolean) (ElapsedSeconds :type Float%20%28double-precision%29) (TriggeredSeconds :type Float%20%28double-precision%29) (InputAction :type Input%20Action%20Object%20Reference :default "/Game/Input/IA_MoveDown.IA_MoveDown"))
  (:Started
    (Utilities|Time|SetGlobalTimeDilation 5.0))
  (:Completed
    (Utilities|Time|SetGlobalTimeDilation 1.0)))

(event Input|EnhancedActionEvents|EnhancedInputActionIA_Move
  (params (ActionValue :type Float%20%28double-precision%29) (ElapsedSeconds :type Float%20%28double-precision%29) (TriggeredSeconds :type Float%20%28double-precision%29) (InputAction :type Input%20Action%20Object%20Reference :default "/Game/Input/IA_Move.IA_Move"))
  (:Started
    (bind _asbp_tetromino (Utilities|Casting|CastToBP_Tetromino (Variables|/Script/BuiltToScale.BlockSpawner|GetActiveBlock (Subsystems|GetBlockSpawner))))
    (Default|TryMove _asbp_tetromino ActionValue)))

(event Input|EnhancedActionEvents|EnhancedInputActionIA_Drop
  (params (ActionValue :type Boolean) (ElapsedSeconds :type Float%20%28double-precision%29) (TriggeredSeconds :type Float%20%28double-precision%29) (InputAction :type Input%20Action%20Object%20Reference :default "/Game/Input/IA_Drop.IA_Drop"))
  (:Started
    (bind _asbp_tetromino (Utilities|Casting|CastToBP_Tetromino (Variables|/Script/BuiltToScale.BlockSpawner|GetActiveBlock (Subsystems|GetBlockSpawner))))
    (Default|LandatDestination _asbp_tetromino)))

(event Input|EnhancedActionEvents|EnhancedInputActionIA_Rotate
  (params (ActionValue :type Float%20%28double-precision%29) (ElapsedSeconds :type Float%20%28double-precision%29) (TriggeredSeconds :type Float%20%28double-precision%29) (InputAction :type Input%20Action%20Object%20Reference :default "/Game/Input/IA_Rotate.IA_Rotate"))
  (:Started
    (bind _asbp_tetromino (Utilities|Casting|CastToBP_Tetromino (Variables|/Script/BuiltToScale.BlockSpawner|GetActiveBlock (Subsystems|GetBlockSpawner))))
    (Default|TryRotate _asbp_tetromino ActionValue)))

(event Input|EnhancedActionEvents|EnhancedInputActionIA_MainMenu
  (params (ActionValue :type Boolean) (ElapsedSeconds :type Float%20%28double-precision%29) (TriggeredSeconds :type Float%20%28double-precision%29) (InputAction :type Input%20Action%20Object%20Reference :default "/Game/Input/IA_MainMenu.IA_MainMenu")))

(event EventBeginPlay
  (bind _returnvalue (PlayerController|LocalPlayerSubsystems|GetEnhancedInputLocalPlayerSubsystem))
  (Utilities|IsValid _returnvalue
    (:Is%20Valid
      (Input|AddMappingContext _returnvalue "/Game/Input/IMC_Default.IMC_Default" 0 "(bIgnoreAllPressedKeysUntilRelease=True,bForceImmediately=False,bNotifyUserSettings=False)"))))

(event EventTick
  (params (DeltaSeconds :type Float%20%28single-precision%29)))

(fn ConstructionScript)