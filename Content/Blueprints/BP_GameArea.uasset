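; BP_GameArea is the playfield of a Tetris-style game, with borders and game-over trigger scaled from SizeX and SizeY.
; On BeginPlay it generates a grid of BP_TriggerPoint actors and hands them to the LineChecker.
; SpawnBlock binds each new tetromino's landing to BlockLanded, which clears lines, fills gaps and spawns the next block.
; A BP_SingleBlock overlapping the top trigger ends the game by opening MainMenu.
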(event OnComponentBeginOverlap(GameOverTrigger)
  (params (OverlappedComponent :type Primitive%20Component%20Object%20Reference) (OtherActor :type Actor%20Object%20Reference) (OtherComp :type Primitive%20Component%20Object%20Reference) (OtherBodyIndex :type Integer) (bFromSweep :type Boolean) (SweepResult :type Hit%20Result%20Structure%20%28by%20ref%29))
  (Utilities|Casting|CastToBP_SingleBlock OtherActor)
  (Game|OpenLevel(byObjectReference) "/Game/Maps/MainMenu.MainMenu"))

(event Custom|SpawnBlock
  (Class|BlockSpawner|SpawnBlock (Subsystems|GetBlockSpawner))
  (bind _asbp_tetromino (Utilities|Casting|CastToBP_Tetromino (Variables|/Script/BuiltToScale.BlockSpawner|GetActiveBlock (Subsystems|GetBlockSpawner))))
  (EventDispatchers|BindEventtoLanding _asbp_tetromino (delegate Custom|BlockLanded)))

(event Custom|BlockLanded
  (bind _returnvalue (Subsystems|GetLineChecker))
  (bind _returnvalue_2 (Class|LineChecker|GetLinestoClean _returnvalue))
  (Class|LineChecker|CleanLines _returnvalue _returnvalue_2)
  (Class|LineChecker|FillEmptyLines _returnvalue _returnvalue_2)
  (CallFunction|SpawnBlock))

(event EventBeginPlay
  (Class|BlueprintTools|GenerateTriggerGrid (Subsystems|GetLineChecker) "/Game/Blueprints/BP_TriggerPoint.BP_TriggerPoint_C" (Variables|Default|GetBottomBorder) 100 (Math|Float|Truncate (Variables|Default|GetSizeX)) (Math|Float|Truncate (Variables|Default|GetSizeY)))
  (bind _outactors (Actor|GetAllActorsOfClass "/Game/Blueprints/BP_TriggerPoint.BP_TriggerPoint_C"))
  (Class|LineChecker|SetTriggerPoints (Subsystems|GetLineChecker) _outactors)
  (CallFunction|ScaleBorders))

(event Collision|EventActorBeginOverlap
  (params (OtherActor :type Actor%20Object%20Reference)))

(event EventTick
  (params (DeltaSeconds :type Float%20%28single-precision%29)))

(fn ConstructionScript
  (CallFunction|ScaleBorders))

(fn ScaleBorders
  (bind _gameovertrigger (Variables|Default|GetGameOverTrigger))
  (Transformation|SetRelativeScale3D (Variables|Default|GetLeftBorder) (Math|Vector|MakeVector 1.0 1.0 (+ (Variables|Default|GetSizeY) 1.0)))
  (Transformation|SetRelativeScale3D (Variables|Default|GetBottomBorder) (Math|Vector|MakeVector 1.0 (Variables|Default|GetSizeX) 1.0))
  (Transformation|SetRelativeLocation (Variables|Default|GetRightBorder) (Math|Vector|MakeVector 0.0 (* (Variables|Default|GetSizeX) 1e+02) 0.0) false false)
  (Transformation|SetRelativeScale3D (Variables|Default|GetRightBorder) (Math|Vector|MakeVector 1.0 1.0 (+ (Variables|Default|GetSizeY) 1.0)))
  (Transformation|SetRelativeLocation _gameovertrigger (Math|Vector|MakeVector 5e+01 (* (Variables|Default|GetSizeX) 5e+01) (+ (* (Variables|Default|GetSizeY) 1e+02) 1e+02)) false false)
  (Transformation|SetRelativeScale3D _gameovertrigger (Math|Vector|MakeVector 1.0 (Variables|Default|GetSizeX) 1.0)))