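; BP_CameraPawn is a camera pawn that frames the BP_GameArea grid through its SpringArm.
; UpdateCameraPosition finds every BP_GameArea, positions the arm on the YZ plane from its SizeX and SizeY, and scales arm length to the larger weighted Y or Z bounds extent.
; The last area found wins, and the function is not called within this Blueprint, whose events are empty.
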(event EventBeginPlay)

(event Collision|EventActorBeginOverlap
  (params (OtherActor :type Actor%20Object%20Reference)))

(event EventTick
  (params (DeltaSeconds :type Float%20%28single-precision%29)))

(fn ConstructionScript)

(fn UpdateCameraPosition
  (bind _springarm (Variables|Default|GetSpringArm))
  (bind _outactors (Actor|GetAllActorsOfClass "/Game/Blueprints/BP_GameArea.BP_GameArea_C"))
  (for _array_element _outactors
    (Transformation|SetWorldLocation _springarm (Math|Vector|MakeVector 0.0 (* (Variables|/Game/Blueprints/BP_GameArea.BP_GameArea_C|GetSizeX _array_element) 5e+01) (+ (* (Variables|/Game/Blueprints/BP_GameArea.BP_GameArea_C|GetSizeY _array_element) 5e+01) 1e+02)) false false)
    (Variables|/Script/Engine.SpringArmComponent|SetTargetArmLength _springarm (Math|Float|Max(Float) (* (.y (.BoxExtent (Collision|GetActorBounds _array_element false false))) 0.9) (* (.z (.BoxExtent (Collision|GetActorBounds _array_element false false))) 2.0)))))