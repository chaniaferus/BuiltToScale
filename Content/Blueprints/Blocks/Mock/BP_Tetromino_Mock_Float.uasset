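; BP_Tetromino_Mock_Float is a mock tetromino block that bobs vertically and rocks in place.
; BeginPlay randomizes phase offsets, frequency and amplitude so each instance moves differently.
; Tick adds a game-time sine to the current Z, without delta-time scaling, and sets roll from a second phase-shifted sine.
; BlockLanding and ProcessBlock are empty, so those events do nothing here.
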(event Custom|ProcessBlock)

(event Custom|BlockLanding)

(event EventBeginPlay
  (Variables|Default|SetRandomOffset (Math|Random|RandomFloatinRange 0.0 1.0))
  (Variables|Default|SetRandomRotOffset (Math|Random|RandomFloatinRange 0.0 1.0))
  (Variables|Default|SetRandomFreq (Math|Random|RandomFloatinRange 0.1 0.25))
  (Variables|Default|SetRandomAplitude (Math|Random|RandomFloatinRange 1.5 2.5)))

(event EventTick
  (params (DeltaSeconds :type Float%20%28single-precision%29))
  (bind _returnvalue (Transformation|GetActorRotation))
  (bind _returnvalue_2 (Transformation|GetActorLocation))
  (bind _returnvalue_3 (Utilities|Time|GetGameTimeinSeconds))
  (bind _randomfreq (Variables|Default|GetRandomFreq))
  (Transformation|SetActorLocation (Math|Vector|MakeVector (.x _returnvalue_2) (.y _returnvalue_2) (+ (.z _returnvalue_2) (* (Variables|Default|GetRandomAplitude) (Math|Trig|Sin(Radians) (* (+ (Variables|Default|GetRandomOffset) _returnvalue_3) _randomfreq))))) false false)
  (Transformation|SetActorRotation (Math|Rotator|MakeRotator (* (Math|Trig|Sin(Radians) (* _randomfreq (+ _returnvalue_3 (Variables|Default|GetRandomRotOffset)))) 15.0) (.pitch _returnvalue) (.yaw _returnvalue))))

(fn ConstructionScript)